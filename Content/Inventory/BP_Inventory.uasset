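; BP_Inventory is an actor that stores items as class-and-amount pairs in a fixed number of slots, sized at BeginPlay.
; AddItem recursively fills partial stacks up to MaxSize, then empty slots, gives non-stackable items one slot each, and returns any remainder.
; Each write refreshes the matching slot widget, and helpers query slots using item class defaults.
; ShowInventory is empty; the widget creation and toggle logic is disconnected.
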(event `self.ReceiveBeginPlay`
  (`KismetArrayLibrary.Array_Resize` (`self.Slots`) (`self.AmountSlots`)))

(event `UpdateSlotIndex`
  (params (Index :type Integer))
  (`/Game/Inventory/UI_InventorySlot.UpdateSlot` (`|GetArrayItem` (`/Game/Inventory/UI_Inventory.SlotsWidget` (`self.InventoryWidget`)) Index)))

(event `ShowInventory`)

(fn `AddItem`
  (params (ItemClass :type "/Game/Item/ItemBase Class Reference") (Amount :type Integer))
  (returns (IsSuccess :type Boolean) (Rest :type Integer))
  (locals (returnClass :type "/Game/Item/ItemBase Class Reference") (returnAmount :type Integer) (FoundIndex :type Integer))
  (bind _foundindex (`local.FoundIndex`))
  (bind _maxsize (`self.MaxSize`))
  (bind _slots (`self.Slots`))
  (bind _foundindex_2 (`local.FoundIndex`))
  (bind _returnclass (`local.returnClass`))
  (bind _returnvalue (+ (`.Amount_8_E6B960C940F1C4247B54B494B4A5BB84` (break `/Game/Inventory/InventorySlot` (`|GetArrayItem` (`self.Slots`) (`local.FoundIndex`)))) (`local.returnAmount`)))
  (set `local.returnClass` ItemClass)
  (set `local.returnAmount` Amount)
  (if (`.canBeStacked_32_3411233C432E1D7673483684DCE8FE82` (break `/Game/Inventory/ItemInfo` (defaults `/Game/Inventory/BP_Inventory` ItemClass)))
    (bind (_issuccess _index) (`self.SearchFreeStack` (`local.returnClass`)))
    (if _issuccess
      (set `local.FoundIndex` _index)
      (if (> _returnvalue _maxsize)
        (set `local.returnAmount` (- _returnvalue _maxsize))
        (`KismetArrayLibrary.Array_Set` _slots _foundindex_2 (make `/Game/Inventory/InventorySlot` _returnclass (`self.MaxSize`)))
        (`self.UpdateSlotIndex` _foundindex_2)
        (bind (_issuccess_2 _rest) (`self.AddItem` _returnclass (`local.returnAmount`)))
        (return true _rest)
        (else
          (`KismetArrayLibrary.Array_Set` _slots _foundindex_2 (make `/Game/Inventory/InventorySlot` _returnclass _returnvalue))
          (`self.UpdateSlotIndex` _foundindex_2)
          (return true 0)))
      (else
        (bind (_issuccess_3 _index_2) (`self.SearchEmptySlot`))
        (if _issuccess_3
          (bind _output_get (set `local.FoundIndex` _index_2))
          (if (> (`local.returnAmount`) (`self.MaxSize`))
            (`KismetArrayLibrary.Array_Set` (`self.Slots`) _output_get (make `/Game/Inventory/InventorySlot` (`local.returnClass`) (`self.MaxSize`)))
            (`self.UpdateSlotIndex` (`local.FoundIndex`))
            (bind (_issuccess_4 _rest_2) (`self.AddItem` (`local.returnClass`) (- (`local.returnAmount`) (`self.MaxSize`))))
            (return true _rest_2)
            (else
              (`KismetArrayLibrary.Array_Set` (`self.Slots`) _foundindex (make `/Game/Inventory/InventorySlot` (`local.returnClass`) (`local.returnAmount`)))
              (`self.UpdateSlotIndex` _foundindex)
              (return true 0)))
          (else
            (return false (`local.returnAmount`))))))
    (else
      (bind (_issuccess_5 _index_3) (`self.SearchEmptySlot`))
      (if _issuccess_5
        (bind _output_get_2 (set `local.FoundIndex` _index_3))
        (`KismetArrayLibrary.Array_Set` (`self.Slots`) _output_get_2 (make `/Game/Inventory/InventorySlot` (`local.returnClass`) 1))
        (`self.UpdateSlotIndex` (`local.FoundIndex`))
        (if (> (`local.returnAmount`) 1)
          (bind (_issuccess_6 _rest_3) (`self.AddItem` (`local.returnClass`) (- (`local.returnAmount`) 1)))
          (return true _rest_3)
          (else
            (return true 0)))
        (else
          (return false (`local.returnAmount`)))))))

(fn `GetAmountIndex`
  (params (Index :type Integer))
  (returns (Amount :type Integer))
  (locals (returnClass :type "/Game/Item/ItemBase Class Reference") (returnAmount :type Integer) (FoundIndex :type Integer))
  (return (`.Amount_8_E6B960C940F1C4247B54B494B4A5BB84` (break `/Game/Inventory/InventorySlot` (`|GetArrayItem` (`self.Slots`) Index)))))

(fn `GetItemInfoIndex`
  (params (Index :type Integer))
  (returns (EmptySlot :type Boolean) (ItemInfo :type "/Game/Inventory/ItemInfo Structure") (Amuont :type Integer))
  (bind (_itemclass _amount) (break `/Game/Inventory/InventorySlot` (`|GetArrayItem` (`self.Slots`) Index)))
  (if (`KismetSystemLibrary.IsValidClass` _itemclass)
    (return false (defaults `/Game/Inventory/BP_Inventory` _itemclass) _amount)
    (else
      (return true (struct) 0))))

(fn `IsSlotEmpty`
  (params (Index :type Integer))
  (returns (IsEmpty :type Boolean))
  (return (not (`KismetSystemLibrary.IsValidClass` (`.ItemClass_7_4F0615E345746AEB5DD4B5932AEC134A` (break `/Game/Inventory/InventorySlot` (`|GetArrayItem` (`self.Slots`) Index)))))))

(fn `SearchEmptySlot`
  (returns (IsSuccess :type Boolean) (Index :type Integer))
  (locals (returnBool :type Boolean) (returnIndex :type Integer))
  (for (_array_element _array_index) (`self.Slots`)
    (if (not (`KismetSystemLibrary.IsValidClass` (`.ItemClass_7_4F0615E345746AEB5DD4B5932AEC134A` (break `/Game/Inventory/InventorySlot` _array_element))))
      (set `local.returnBool` true)
      (set `local.returnIndex` _array_index)
      (break)))
  (return (`local.returnBool`) (`local.returnIndex`)))

(fn `SearchFreeStack`
  (params (ItemClass :type "/Game/Item/ItemBase Class Reference"))
  (returns (IsSuccess :type Boolean) (Index :type Integer))
  (locals (returnBool :type Boolean) (returnIndex :type Integer))
  (for (_array_element _array_index) (`self.Slots`)
    (bind (_itemclass _amount) (break `/Game/Inventory/InventorySlot` _array_element))
    (if (`KismetSystemLibrary.IsValidClass` _itemclass)
      (if (and (== _itemclass ItemClass) (< _amount (`self.MaxSize`)))
        (set `local.returnBool` true)
        (set `local.returnIndex` _array_index)
        (break))))
  (return (`local.returnBool`) (`local.returnIndex`)))

(fn `UserConstructionScript`)