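; Enemy2 is a melee enemy character that chases and attacks the player, takes damage, and dies.
; Tick caches player distance, direction and death status, then drives an enum state machine that idles, follows or attacks by range.
; Attack events repeat the montage or resume the chase, and toggle a capsule hitbox that applies damage on overlap.
; At zero HP it plays a death montage, disables collision and destroys itself after a delay.
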(event `self.ReceiveTick`
  (params (DeltaSeconds :type "Float (single-precision)"))
  (`self.SaveDisAndDir`)
  (if (`self.IsDeathPlayerChar`)
    (set `self.CurState` "NewEnumerator3"))
  (switch `/Game/Enums/MonsterState` (`self.CurState`)
    (:`NewEnumerator0`
      (if (<= (`self.DistancePlayerChar`) 500.0)
        (set `self.CurState` "NewEnumerator1")))
    (:`NewEnumerator1`
      (if (<= (`self.DistancePlayerChar`) 160.0)
        (set `self.CurState` "NewEnumerator2")
        (`self.PlayAnimMontage` "/Game/ModularRPGHeroesPolyart/Animations/SwordAndShieldStance/NormalAttack01_SwordShieldAnim_Montage.NormalAttack01_SwordShieldAnim_Montage")
        (set `self.IsAttacking` true)
        (else
          (`self.AddMovementInput` (`self.DirToPlayerChar`)))))
    (:`NewEnumerator2`
      (if (`self.IsAttacking`)
        _
        (elif (> (`self.DistancePlayerChar`) 180.0)
          (set `self.CurState` "NewEnumerator1"))))))

(event `OnAnimEnd_Attack`
  (set `self.IsAttacking` false)
  (if (`self.IsDeathPlayerChar`)
    (set `self.CurState` "NewEnumerator3")
    (elif (> (`self.DistancePlayerChar`) 180.0)
      (set `self.CurState` "NewEnumerator1")
      (else
        (`self.PlayAnimMontage` "/Game/ModularRPGHeroesPolyart/Animations/SwordAndShieldStance/NormalAttack01_SwordShieldAnim_Montage.NormalAttack01_SwordShieldAnim_Montage")
        (set `self.IsAttacking` true)))))

(event `SaveDisAndDir`
  (bind _returnvalue (`GameplayStatics.GetPlayerCharacter` 0))
  (bind _returnvalue_2 (- (`self.K2_GetActorLocation` _returnvalue) (`self.K2_GetActorLocation`)))
  (bind _asmain_player_character (cast `/Game/Player/MainPlayerCharacter` _returnvalue))
  (set `self.IsDeathPlayerChar` (`/Game/Player/MainPlayerCharacter.IsDeath` _asmain_player_character))
  (set `self.DistancePlayerChar` (`KismetMathLibrary.VSize` _returnvalue_2))
  (set `self.DirToPlayerChar` (`KismetMathLibrary.Normal` _returnvalue_2)))

(event `OnColStart_Attack`
  (`PrimitiveComponent.SetCollisionEnabled` (`self.Capsule`) "QueryAndPhysics"))

(event `OnColEnd_Attack`
  (`PrimitiveComponent.SetCollisionEnabled` (`self.Capsule`) "NoCollision"))

(event `self.Capsule.OnComponentBeginOverlap`
  (params (OverlappedComponent :type "PrimitiveComponent Object Reference") (OtherActor :type "Actor Object Reference") (OtherComp :type "PrimitiveComponent Object Reference") (OtherBodyIndex :type Integer) (bFromSweep :type Boolean) (SweepResult :type "HitResult Structure (by ref)"))
  (if (!= OtherActor self)
    (`GameplayStatics.ApplyDamage` OtherActor (`self.Atk`) null self)))

(event `self.ReceiveAnyDamage`
  (params (Damage :type "Float (single-precision)") (DamageType :type "DamageType Object Reference") (InstigatedBy :type "Controller Object Reference") (DamageCauser :type "Actor Object Reference"))
  (bind _output_get (set `self.Hp` (- (`self.Hp`) Damage)))
  (if (<= _output_get 0.0)
    (`self.PlayAnimMontage` "/Game/ModularRPGHeroesPolyart/Animations/SwordAndShieldStance/Die_SwordShieldAnim_Montage.Die_SwordShieldAnim_Montage")
    (set `self.CurState` "NewEnumerator4")
    (`PrimitiveComponent.SetCollisionEnabled` (`self.CapsuleComponent`) "NoCollision")
    (`PrimitiveComponent.SetCollisionEnabled` (`self.Capsule`) "NoCollision")
    (`KismetSystemLibrary.Delay` 2.0)
    (`self.K2_DestroyActor`)))

(fn `UserConstructionScript`)